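; Level exit door that opens once the player collects enough coins, then leads to the next level.
; Tick polls the GameInstance coin count against PointsToOpen, rotating the actor and playing a one-time opening sound on a match.
; Character overlap with the open door plays a fade-out sequence, resets coins and loads NextLevel.
; Interact plays a one-time locked sound, checking a hardcoded 15 instead of PointsToOpen.
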(event OnComponentBeginOverlap(Box)
  (params (OverlappedComponent :type Primitive%20Component%20Object%20Reference) (OtherActor :type Actor%20Object%20Reference) (OtherComp :type Primitive%20Component%20Object%20Reference) (OtherBodyIndex :type Integer) (bFromSweep :type Boolean) (SweepResult :type Hit%20Result%20Structure%20%28by%20ref%29))
  ;[0.15 0.15 0.15 0.5] Load Level
  (Utilities|Casting|CastToBP_ThirdPersonCharacter OtherActor)
  (if (Variables|Default|GetIsOpened)
    (bind _outactor (Sequencer|Player|CreateLevelSequencePlayer "/Game/Game/VFX/Cinematic/LS_FadeOut.LS_FadeOut"))
    (Sequencer|Player|Play (Variables|/Script/LevelSequence.LevelSequenceActor|GetSequencePlayer _outactor) :!class /Script/MovieScene.MovieSceneSequencePlayer)
    (Utilities|FlowControl|Delay 1.5)
    (bind _asbp_game_instance (Utilities|Casting|CastToBP_GameInstance (Game|GetGameInstance)))
    (Variables|/Game/Game/Blueprints/BP_GameInstance.BP_GameInstance_C|SetTotalCoinsPickupLevel _asbp_game_instance 0)
    (Game|OpenLevel(byObjectReference) (Variables|Default|GetNextLevel))))

(event EventBeginPlay)

(event Collision|EventActorBeginOverlap
  (params (OtherActor :type Actor%20Object%20Reference)))

(event EventTick
  (params (DeltaSeconds :type Float%20%28single-precision%29))
  ;[0.15 0.15 0.15 0.5] Opening after 15points
  (bind _asbp_game_instance (Utilities|Casting|CastToBP_GameInstance (Game|GetGameInstance)))
  (bind _output_get (Variables|Default|SetGameInstanceRef _asbp_game_instance))
  (if (== (Variables|/Game/Game/Blueprints/BP_GameInstance.BP_GameInstance_C|GetTotalCoinsPickupLevel _output_get) (Variables|Default|GetPointsToOpen))
    (Transformation|SetActorRotation (Components|GetOwner (Variables|Default|GetDoor)) "0.000000,-70.000000,0.000000")
    (Utilities|FlowControl|DoOnce false
      (:Completed
        (Audio|PlaySoundatLocation "/Game/Game/Audio/SFX/S_OpeningDoor_Cue.S_OpeningDoor_Cue" (Transformation|GetActorLocation self) "0, 0, 0" 1.0 1.0 0.0 0 0 0 0)
        (Variables|Default|SetIsOpened true)))))

(event EventInteract
  ;[0.15 0.15 0.15 0.5] Lock before 15points
  (bind _asbp_game_instance (Utilities|Casting|CastToBP_GameInstance (Game|GetGameInstance)))
  (bind _output_get (Variables|Default|SetGameInstanceRef _asbp_game_instance))
  (if (not (== (Variables|/Game/Game/Blueprints/BP_GameInstance.BP_GameInstance_C|GetTotalCoinsPickupLevel _output_get) 15))
    (Utilities|FlowControl|DoOnce false
      (:Completed
        (Audio|PlaySoundatLocation "/Game/Game/Audio/SFX/S_LockedDoor_Cue.S_LockedDoor_Cue" (Transformation|GetActorLocation self) "0, 0, 0" 1.0 1.0 0.0 0 0 0 0)))))

(fn ConstructionScript)