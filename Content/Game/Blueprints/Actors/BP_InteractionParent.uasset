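; Base interactable actor that registers itself with BP_ThirdPersonCharacter while the character overlaps its sphere trigger.
; The construction script applies configurable variables to the mesh, trigger radius and location, and UI component position.
; Begin and end overlap call AddInteraction and RemoveInteraction on the character, and ToggleUI exposes the UI's visibility.
; Interact stores the passed Character and only prints a debug message as a placeholder.
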(event OnComponentBeginOverlap(interactTrigger)
  (params (OverlappedComponent :type Primitive%20Component%20Object%20Reference) (OtherActor :type Actor%20Object%20Reference) (OtherComp :type Primitive%20Component%20Object%20Reference) (OtherBodyIndex :type Integer) (bFromSweep :type Boolean) (SweepResult :type Hit%20Result%20Structure%20%28by%20ref%29))
  (bind _asbp_third_person_character (Utilities|Casting|CastToBP_ThirdPersonCharacter OtherActor))
  (Default|AddInteraction _asbp_third_person_character self))

(event OnComponentEndOverlap(interactTrigger)
  (params (OverlappedComponent :type Primitive%20Component%20Object%20Reference) (OtherActor :type Actor%20Object%20Reference) (OtherComp :type Primitive%20Component%20Object%20Reference) (OtherBodyIndex :type Integer))
  (bind _asbp_third_person_character (Utilities|Casting|CastToBP_ThirdPersonCharacter OtherActor))
  (Default|RemoveInteraction _asbp_third_person_character self))

(fn ConstructionScript
  (setup|SetupMesh)
  (Setup|SetupTrigger)
  (Setup|SetupUI))

(fn SetupMesh
  (Components|StaticMesh|SetStaticMesh (Variables|Default|GetinteractMesh) (Variables|Setup|GetInteractionMesh))
  (Transformation|SetRelativeTransform (Variables|Default|GetinteractMesh) (Variables|setup|GetMeshTransfrom) false false))

(fn SetupTrigger
  (Components|Sphere|SetSphereRadius (Variables|Default|GetinteractTrigger) (Variables|Setup|GetTriggerRadius) true)
  (Transformation|SetRelativeLocation (Variables|Default|GetinteractTrigger) (Variables|Setup|GetTriggerLocation) false false))

(fn SetupUI
  (Transformation|SetRelativeLocation (Variables|Default|GetinteractUi) (Variables|Setup|GetUILocation) false false))

(fn ToggleUI
  (params (BeVisible :type Boolean))
  (Rendering|SetVisibility (Variables|Default|GetinteractUi) BeVisible false))

(fn Interact
  (params (Character :type BP%20Third%20Person%20Character%20Object%20Reference))
  (Variables|Default|SetCharacter Character)
  (Development|PrintString "INTERACTED"))