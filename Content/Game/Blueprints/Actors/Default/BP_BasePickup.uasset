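; Base pickup actor that damages or heals the player on overlapping its box, depending on the sign of HealthChangeAmount.
; The overlapping third-person character's player state supplies the health component that receives the change.
; An invincible player is ignored for both damage and healing, and damage makes the player invincible.
; Each sound plays once per instance through DoOnce, and DestroyActor optionally removes the pickup after use.
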(event OnComponentBeginOverlap(Box)
  (params (OverlappedComponent :type Primitive%20Component%20Object%20Reference) (OtherActor :type Actor%20Object%20Reference) (OtherComp :type Primitive%20Component%20Object%20Reference) (OtherBodyIndex :type Integer) (bFromSweep :type Boolean) (SweepResult :type Hit%20Result%20Structure%20%28by%20ref%29))
  (bind _asbp_third_person_character (Utilities|Casting|CastToBP_ThirdPersonCharacter OtherActor))
  (bind _output_get (Variables|Default|SetPlayerRef _asbp_third_person_character))
  (bind _asbp_player_state (Utilities|Casting|CastToBP_PlayerState (Variables|/Script/Engine.Pawn|GetPlayerState _output_get)))
  (if (not (Variables|/Game/Game/Blueprints/Pawns_Characters/Player/BP_ThirdPersonCharacter.BP_ThirdPersonCharacter_C|GetIsInvincible (Variables|Default|GetPlayerRef)))
    (if (< (Variables|Health/Damage|GetHealthChangeAmount) 0.0)
      (Default|TakeDamage (Variables|/Game/Game/Blueprints/PlayerStates/BP_PlayerState.BP_PlayerState_C|GetAC_Health _asbp_player_state) (Math|Float|Absolute(Float) (Variables|Health/Damage|GetHealthChangeAmount)))
      (Variables|/Game/Game/Blueprints/Pawns_Characters/Player/BP_ThirdPersonCharacter.BP_ThirdPersonCharacter_C|SetIsInvincible (Variables|Default|GetPlayerRef) true)
      (Utilities|FlowControl|DoOnce false
        (:Completed
          (Audio|PlaySound2D "/Game/Game/Audio/SFX/player-hurt_Cue.player-hurt_Cue" 1.0 1.0 0.0 0 0)))
      (else
        (Default|GainHealth (Variables|/Game/Game/Blueprints/PlayerStates/BP_PlayerState.BP_PlayerState_C|GetAC_Health _asbp_player_state) (Variables|Health/Damage|GetHealthChangeAmount))
        (Utilities|FlowControl|DoOnce false
          (:Completed
            (Audio|PlaySound2D "/Game/Game/Audio/SFX/heal-pickup_Cue.heal-pickup_Cue" 1.0 1.0 0.0 0 0)))))
    (if (Variables|Health/Damage|GetDestroyActor)
      (Actor|DestroyActor))))

(fn ConstructionScript)